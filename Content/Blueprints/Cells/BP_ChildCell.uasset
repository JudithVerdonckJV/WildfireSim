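; Cell Blueprint that provides the fire visual effect for a single cell on the terrain.
; HandleFireVFX switches the Fire effect component on or off, resetting it and matching its visibility to the active state.
; SetFireRotationandLocation teleports Fire to the cell's terrain intersection point and rotation, then sets its FireRadius user parameter to half the cell size.
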(event `self.HandleFireVFX`
  (params (activate :type Boolean))
  (bind _fire (`self.Fire`))
  (`ActorComponent.SetActive` _fire activate true)
  (`SceneComponent.SetVisibility` _fire activate false))

(event `self.SetFireRotationAndLocation`
  (`SceneComponent.K2_SetWorldLocationAndRotation` (`self.Fire`) (`self.TerrainIntersectionPoint`) (`self.TerrainIntersectionRotation`) false true)
  (`FXSystemComponent.SetFloatParameter` (`self.Fire`) "User.FireRadius" (/ (`self.CellSize`) 2.0)))

(fn `UserConstructionScript`)