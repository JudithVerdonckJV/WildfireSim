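; BP_Observer is the player's orbit-camera viewer for a simulator with ignition points and wind-affected cells.
; On BeginPlay it creates the WID_Simulator UI with itself as owner and spawns hidden ignition-point and selected-cell marker actors.
; Input rotates the spring arm while Move is held and zooms it within clamped limits.
; Events reposition, show or update these reused markers, including cell extents and wind velocity; only the ignition marker can be re-hidden.
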(event `self.ReceiveBeginPlay`
  (bind _returnvalue (`|CreateWidget` "/Game/Blueprints/UI/WID_Simulator.WID_Simulator_C" (`GameplayStatics.GetPlayerController` 0)))
  (bind _output_get (set `self.UI` _returnvalue))
  (`/Game/Blueprints/UI/WID_Simulator.SetOwner` _output_get self)
  (`UserWidget.AddToViewport` _output_get 0)
  (bind _returnvalue_2 (`|SpawnActorFromClass` "/Game/Blueprints/Observer/BP_IgnitionPoint.BP_IgnitionPoint_C" (`KismetMathLibrary.MakeTransform` (0.0 0.0 0.0)) "Undefined" "OverrideRootScale" null null))
  (bind _output_get_2 (set `self.IgnitionPointActor` _returnvalue_2))
  (`self.SetActorTickEnabled` _output_get_2 false)
  (`self.SetActorHiddenInGame` _output_get_2 true)
  (bind _returnvalue_3 (`|SpawnActorFromClass` "/Game/Blueprints/Observer/BP_SelectedCell.BP_SelectedCell_C" (`KismetMathLibrary.MakeTransform` (0.0 0.0 0.0)) "Undefined" "OverrideRootScale" null null))
  (bind _output_get_3 (set `self.SelectedCellActor` _returnvalue_3))
  (`self.SetActorTickEnabled` _output_get_3 false)
  (`self.SetActorHiddenInGame` _output_get_3 true))

(event `InputAxis|Move`
  (params (AxisValue :type "Float (single-precision)"))
  ;[1 1 1] Viewport navigation
  (set `self.bCanMove` (> AxisValue 0.1)))

(event `InputVectorAxis|Mouse2D`
  (params (AxisValue :type "Vector Structure"))
  (bind (_returnvalue_x _returnvalue_y) (`KismetMathLibrary.BreakVector` (* AxisValue (`self.RotationSpeed`))))
  ;[1 1 1] Viewport navigation
  (if (`self.bCanMove`)
    (`SceneComponent.K2_AddLocalRotation` (`self.SpringArm`) (`KismetMathLibrary.MakeRotator` 0.0 _returnvalue_y _returnvalue_x) false false)))

(event `InputAxis|Scroll`
  (params (AxisValue :type "Float (single-precision)"))
  (bind _springarm (`self.SpringArm`))
  ;[1 1 1] Viewport navigation
  (if (> (`KismetMathLibrary.Abs` AxisValue) 0.1)
    (set `SpringArmComponent.TargetArmLength` (`KismetMathLibrary.FClamp` (+ (`SpringArmComponent.TargetArmLength` _springarm) (* (`self.ZoomSpeed`) AxisValue)) (`self.ZoomMin`) (`self.ZoomMax`)) _springarm)))

(event `HideIgnitionPoint`
  (bind _ignitionpointactor (`self.IgnitionPointActor`))
  (`self.SetActorTickEnabled` _ignitionpointactor false)
  (`self.SetActorHiddenInGame` _ignitionpointactor true))

(event `self.SetIgnitionPoint_VFX`
  (params (location :type "Vector Structure (by ref)") (rotation :type "Rotator Structure (by ref)"))
  (bind _ignitionpointactor (`self.IgnitionPointActor`))
  ;[1 1 1] Ignition point
  (`self.SetActorTickEnabled` _ignitionpointactor true)
  (`self.SetActorHiddenInGame` _ignitionpointactor false)
  (`self.K2_SetActorLocationAndRotation` _ignitionpointactor location rotation false false))

(event `self.SetSelectedCellVisual`
  (params (location :type "Vector Structure (by ref)") (halfextents :type "Vector Structure (by ref)") (windDirection :type "Vector Structure (by ref)"))
  (bind _selectedcellactor (`self.SelectedCellActor`))
  ;[1 1 1] Selection
  (`self.SetActorHiddenInGame` _selectedcellactor false)
  (`self.K2_SetActorLocation` _selectedcellactor location false true)
  (`/Game/Blueprints/Observer/BP_SelectedCell.SetHalfExtents` _selectedcellactor halfextents)
  (`/Game/Blueprints/Observer/BP_SelectedCell.SetWindVelocity` _selectedcellactor windDirection))

(event `self.UpdateWindVelocityVisual`
  (params (windVel :type "Vector Structure (by ref)"))
  (`/Game/Blueprints/Observer/BP_SelectedCell.SetWindVelocity` (`self.SelectedCellActor`) windVel))

(fn `UserConstructionScript`)